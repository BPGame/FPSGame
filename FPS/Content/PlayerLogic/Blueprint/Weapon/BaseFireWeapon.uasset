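; Base firearm Blueprint for the player, handling firing, clip and reserve ammo, reloading and scope controls.
; Attack fires immediately and, with AutoFire, repeats Fire on a looping timer until StopAttack or an empty clip.
; Each shot spends ammo, spawns a projectile and plays montage, muzzle, shell, sound and camera-shake effects.
; Scope events forward to a BP_ScopeMaster child actor cached on BeginPlay; InspectWeapon triggers Reload, which refills from reserve.
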(event Custom|ScopeZoom
  (params (Condition :type Boolean))
  (if Condition
    (Default|ScopeZoom (Variables|Default|GetScopeReference) false)
    (else
      (Default|ScopeZoom (Variables|Default|GetScopeReference) true))))

(event Custom|TargetScope
  (Default|CycleScopes (Variables|Default|GetScopeReference)))

(event Custom|SwitchScope
  (Default|SwitchScopeType (Variables|Default|GetScopeReference)))

(event EventBeginPlay
  (bind _asbp_scope_master (Utilities|Casting|CastToBP_ScopeMaster (Variables|/Script/Engine.ChildActorComponent|GetChildActor (Variables|Default|GetScope))))
  (Variables|Default|SetScopeReference _asbp_scope_master))

(event EventAttack
  (CallFunction|Fire)
  (if (Variables|Default|GetAutoFire)
    (bind _returnvalue (Utilities|Time|SetTimerbyFunctionName self "Fire" (Variables|Default|GetSpeedFire) true))
    (Variables|Default|SetFireTimer _returnvalue)))

(event EventStopAttack
  (Utilities|Time|ClearandInvalidateTimerbyHandle (Variables|Default|GetFireTimer)))

(event EventInspectWeapon
  (CallFunction|Reload))

(fn ConstructionScript
  (|CallParentFunction))

(fn Fire
  (bind _weaponmesh (Variables|Default|GetWeaponMesh))
  (bind _weaponmesh_2 (Variables|Default|GetWeaponMesh))
  (bind _returnvalue (Transformation|GetSocketLocation _weaponmesh_2 "MuzzleSocket"))
  (bind _returnvalue_2 (Transformation|GetSocketRotation _weaponmesh_2 "MuzzleSocket"))
  (if (CallFunction|CalculateAmmo)
    (Animation|PlayAnimMontage (Game|GetPlayerCharacter 0) (Variables|Default|GetFireMontage) 1.0 "None")
    (Game|SpawnActorfromClass (Variables|Default|GetBulletClass) (Math|Transform|MakeTransform _returnvalue _returnvalue_2 "1,1,1") "Undefined" 0 0)
    (Effects|SpawnEmitteratLocation (Variables|Default|GetEmitter%20Muzzle) _returnvalue _returnvalue_2)
    (Effects|SpawnEmitteratLocation (Variables|Default|GetEmitter%20Shell) (Transformation|GetSocketLocation _weaponmesh "ShellEjectionSocket") (Transformation|GetSocketRotation _weaponmesh "ShellEjectionSocket"))
    (Audio|PlaySoundatLocation (Variables|Default|GetFireSound) (Transformation|GetSocketLocation (Variables|Default|GetWeaponMesh) "MuzzleSocket") "0, 0, 0" 1.0 1.0 0.0 0 0 0)
    (Game|Feedback|ClientStartCameraShake (Game|GetPlayerController 0) "/Game/PlayerLogic/Blueprint/Weapon/BallisticsVFX/FirstPersonBPExamples/HeadBobShake.HeadBobShake_C" 1.0 "CameraLocal" "0, 0, 0")
    (else
      (Audio|PlaySoundatLocation (Variables|Default|GetNoAmmoSound) (Transformation|GetSocketLocation (Variables|Default|GetWeaponMesh) "MuzzleSocket") "0, 0, 0" 1.0 1.0 0.0 0 0 0)
      (CallFunction|StopAttack))))

(fn CalculateAmmo
  (if (> (Variables|Default|GetCurrentAmmoInClip) 0)
    (Variables|Default|SetCurrentAmmoInClip (- (Variables|Default|GetCurrentAmmoInClip) 1))
    (return true)
    (else
      (return false))))

(fn Reload
  (if (> (Variables|Default|GetCurrentAmmoInClip) 0)
    (Variables|Default|SetBaseAmmo (+ (Variables|Default|GetCurrentAmmoInClip) (Variables|Default|GetBaseAmmo))))
  (if (> (Variables|Default|GetBaseAmmo) (Variables|Default|GetMaxAmmoInClip))
    (bind _output_get (Variables|Default|SetCurrentAmmoInClip (Variables|Default|GetMaxAmmoInClip)))
    (Variables|Default|SetBaseAmmo (- (Variables|Default|GetBaseAmmo) _output_get))
    (else
      (Variables|Default|SetCurrentAmmoInClip (Variables|Default|GetBaseAmmo))
      (Variables|Default|SetBaseAmmo 0))))