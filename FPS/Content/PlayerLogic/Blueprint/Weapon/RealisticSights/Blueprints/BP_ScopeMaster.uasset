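; Master weapon scope Blueprint that builds either a transparent sight or a magnified distanced scope from DataTable rows.
; Construction and update events load the row, create the mesh and push its settings into a dynamic material.
; Distanced scopes add a socket-attached SceneCapture2D, whose FOV a timeline lerps in clamped zoom steps.
; Events cycle rows or switch type and table; the demo-only settings clamp is disconnected.
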(event Custom|Scope_Zoom
  (params (ZoomIn :type Boolean))
  (|UpdateFieldOfView ZoomIn))

(event Custom|Update_Scope
  (params (ScopeType :type Enum_ScopeType%20Enum :default "NewEnumerator0") (ScopeDataTable :type Data%20Table%20Row%20Handle%20Structure))
  (|HandleUpdateScope ScopeType ScopeDataTable))

(event Custom|Switch_Scope_Type
  (|HandleSwitchScopeType))

(event Custom|Cycle_Scopes
  (|HandleCycleScopes))

(fn ConstructionScript
  ;[0 0 0 1 16] It's Also Expensive To Change Each Of The Values On Construct. Update Parameters Separately Only When You Need.
  (CallFunction|UpdateScope (Variables|ScopeSettings|GetScopeType) (Variables|ScopeSettings|GetScopeDataTable)))

(fn UpdateTransparentScope
  (bind _transparentscopesettings (Variables|ScopeSettings|GetTransparentScopeSettings))
  (bind _transparentscopesettings_2 (Variables|ScopeSettings|GetTransparentScopeSettings))
  (bind _transparentscopesettings_3 (Variables|ScopeSettings|GetTransparentScopeSettings))
  (bind _transparentscopesettings_4 (Variables|ScopeSettings|GetTransparentScopeSettings))
  (bind _dirtsettings (Utilities|Struct|BreakStruct_MasterTransparentScope _transparentscopesettings_3))
  (bind (_glassopacity _glasscolor) (Utilities|Struct|BreakStruct_MasterTransparentScope _transparentscopesettings_4))
  (bind _sightsettings (Utilities|Struct|BreakStruct_MasterTransparentScope _transparentscopesettings))
  (bind _fadesettings (Utilities|Struct|BreakStruct_MasterTransparentScope _transparentscopesettings_2))
  (bind (_bumpoffset _emissivepower _sightrotation _sightscale _sightredcolor _sightbluecolor _sightgreencolor _sightposition _sighttexture) (Utilities|Struct|BreakStruct_TScopeSight _sightsettings))
  (bind (_fadeposition _fadedensity) (Utilities|Struct|BreakStruct_TScopeFade _fadesettings))
  (bind (_dirtmaskvisibility _dirtpower _dirtrotation _dirtscale _dirtposition _dirttexture) (Utilities|Struct|BreakStruct_TScopeDirt _dirtsettings))
  (bind (_left _right _top _bottom) (Utilities|Struct|BreakStruct_MarginAdv _fadeposition))
  (bind (_x _y) (Math|Vector2D|BreakVector2D _dirtposition))
  (bind (_x_2 _y_2) (Math|Vector2D|BreakVector2D _sightposition))
  ;[0 0 0 1 16] Create Dynamic Material
  (CallFunction|CreateScopeMesh)
  (CallFunction|CreateDynamicMaterial)
  ;[0 0 0 1 16] Update Glass
  (Rendering|Material|SetScalarParameterValue (Variables|DynamicMaterials|GetScopeDynamicMaterial) "Glass Opacity" _glassopacity :!class /Script/Engine.MaterialInstanceDynamic)
  (Rendering|Material|SetVectorParameterValue (Variables|DynamicMaterials|GetScopeDynamicMaterial) "Glass Color" _glasscolor :!class /Script/Engine.MaterialInstanceDynamic)
  ;[0 0 0 1 16] Update Sight
  (Rendering|Material|SetScalarParameterValue (Variables|DynamicMaterials|GetScopeDynamicMaterial) "Bump Offset" _bumpoffset :!class /Script/Engine.MaterialInstanceDynamic)
  (Rendering|Material|SetScalarParameterValue (Variables|DynamicMaterials|GetScopeDynamicMaterial) "Emissive Power" _emissivepower :!class /Script/Engine.MaterialInstanceDynamic)
  (Rendering|Material|SetScalarParameterValue (Variables|DynamicMaterials|GetScopeDynamicMaterial) "Sight Rotation" (Demo|SelectRotation _sightrotation) :!class /Script/Engine.MaterialInstanceDynamic)
  (Rendering|Material|SetScalarParameterValue (Variables|DynamicMaterials|GetScopeDynamicMaterial) "Sight Scale" _sightscale :!class /Script/Engine.MaterialInstanceDynamic)
  (Rendering|Material|SetVectorParameterValue (Variables|DynamicMaterials|GetScopeDynamicMaterial) "Sight Red Color" _sightredcolor :!class /Script/Engine.MaterialInstanceDynamic)
  (Rendering|Material|SetVectorParameterValue (Variables|DynamicMaterials|GetScopeDynamicMaterial) "Sight Blue Color" _sightbluecolor :!class /Script/Engine.MaterialInstanceDynamic)
  (Rendering|Material|SetVectorParameterValue (Variables|DynamicMaterials|GetScopeDynamicMaterial) "Sight Green Color" _sightgreencolor :!class /Script/Engine.MaterialInstanceDynamic)
  (Rendering|Material|SetScalarParameterValue (Variables|DynamicMaterials|GetScopeDynamicMaterial) "Sight Position X" _x_2 :!class /Script/Engine.MaterialInstanceDynamic)
  (Rendering|Material|SetScalarParameterValue (Variables|DynamicMaterials|GetScopeDynamicMaterial) "Sight Position Y" _y_2 :!class /Script/Engine.MaterialInstanceDynamic)
  (Rendering|Material|SetTextureParameterValue (Variables|DynamicMaterials|GetScopeDynamicMaterial) "Sight Texture" _sighttexture)
  ;[0 0 0 1 16] Update Fade Settings
  (Rendering|Material|SetScalarParameterValue (Variables|DynamicMaterials|GetScopeDynamicMaterial) "Fade Density" _fadedensity :!class /Script/Engine.MaterialInstanceDynamic)
  (Rendering|Material|SetScalarParameterValue (Variables|DynamicMaterials|GetScopeDynamicMaterial) "Left Fade Position" _left :!class /Script/Engine.MaterialInstanceDynamic)
  (Rendering|Material|SetScalarParameterValue (Variables|DynamicMaterials|GetScopeDynamicMaterial) "Right Fade Position" _right :!class /Script/Engine.MaterialInstanceDynamic)
  (Rendering|Material|SetScalarParameterValue (Variables|DynamicMaterials|GetScopeDynamicMaterial) "Top Fade Position" _top :!class /Script/Engine.MaterialInstanceDynamic)
  (Rendering|Material|SetScalarParameterValue (Variables|DynamicMaterials|GetScopeDynamicMaterial) "Bottom Fade Position" _bottom :!class /Script/Engine.MaterialInstanceDynamic)
  ;[0 0 0 1 16] Update Dirt Mask
  (Rendering|Material|SetScalarParameterValue (Variables|DynamicMaterials|GetScopeDynamicMaterial) "Dirt Mask Visibility" _dirtmaskvisibility :!class /Script/Engine.MaterialInstanceDynamic)
  (Rendering|Material|SetScalarParameterValue (Variables|DynamicMaterials|GetScopeDynamicMaterial) "Dirt Power" _dirtpower :!class /Script/Engine.MaterialInstanceDynamic)
  (Rendering|Material|SetScalarParameterValue (Variables|DynamicMaterials|GetScopeDynamicMaterial) "Dirt Rotation" (Demo|SelectRotation _dirtrotation) :!class /Script/Engine.MaterialInstanceDynamic)
  (Rendering|Material|SetScalarParameterValue (Variables|DynamicMaterials|GetScopeDynamicMaterial) "Dirt Scale" _dirtscale :!class /Script/Engine.MaterialInstanceDynamic)
  (Rendering|Material|SetScalarParameterValue (Variables|DynamicMaterials|GetScopeDynamicMaterial) "Dirt Position X" _x :!class /Script/Engine.MaterialInstanceDynamic)
  (Rendering|Material|SetScalarParameterValue (Variables|DynamicMaterials|GetScopeDynamicMaterial) "Dirt Position Y" _y :!class /Script/Engine.MaterialInstanceDynamic)
  (Rendering|Material|SetTextureParameterValue (Variables|DynamicMaterials|GetScopeDynamicMaterial) "Dirt Texture" _dirttexture))

(fn ClampSightSettings
  (bind _transparentscopesettings (Variables|ScopeSettings|GetTransparentScopeSettings))
  (bind _transparentscopesettings_2 (Variables|ScopeSettings|GetTransparentScopeSettings))
  (bind _transparentscopesettings_3 (Variables|ScopeSettings|GetTransparentScopeSettings))
  (bind _glassopacity (Utilities|Struct|BreakStruct_MasterTransparentScope _transparentscopesettings))
  (bind _dirtsettings (Utilities|Struct|BreakStruct_MasterTransparentScope _transparentscopesettings_2))
  (bind _sightsettings (Utilities|Struct|BreakStruct_MasterTransparentScope _transparentscopesettings_3))
  (bind (_emissivepower _sightrotation _sightscale) (Utilities|Struct|BreakStruct_TScopeSight _sightsettings))
  (bind (_dirtmaskvisibility _dirtrotation _dirtscale) (Utilities|Struct|BreakStruct_TScopeDirt _dirtsettings))
  ;[0 0 0 1 16] Keep Glass Opacity Between 0.1 And 1.
  (Utilities|Struct|SetmembersinStruct_MasterTransparentScope _transparentscopesettings (select (<= _glassopacity 0.1) 0.1 (select (>= _glassopacity 1.0) 1.0 _glassopacity)))
  ;[0 0 0 1 16] Keep Sight Rotation Between -180 And 180 | Keep Scale And Emissive Power Higher Than 0
  (bind _structout (Utilities|Struct|SetmembersinStruct_TScopeSight _sightsettings (select (<= _emissivepower 0.0) 0.0 _emissivepower) (select (>= _sightrotation 1.8e+02) 1.8e+02 (select (<= _sightrotation -1.8e+02) -1.8e+02 _sightrotation)) (select (<= _sightscale 0.0) 0.1 _sightscale)))
  (Utilities|Struct|SetmembersinStruct_MasterTransparentScope (Variables|ScopeSettings|GetTransparentScopeSettings) _structout)
  ;[0 0 0 1 16] Keep Sight Rotation Between -180 And 180 | Keep Scale And Emissive Power Higher Than 0
  (bind _structout_2 (Utilities|Struct|SetmembersinStruct_TScopeDirt _dirtsettings (select (<= _dirtmaskvisibility 0.0) 0.0 (select (>= _dirtmaskvisibility 1.0) 1.0 _dirtmaskvisibility)) (select (>= _dirtrotation 1.8e+02) 1.8e+02 (select (<= _dirtrotation -1.8e+02) -1.8e+02 _dirtrotation)) (select (<= _dirtscale 0.0) 0.1 _dirtscale)))
  (Utilities|Struct|SetmembersinStruct_MasterTransparentScope (Variables|ScopeSettings|GetTransparentScopeSettings) _structout_2))

(fn SelectRotation
  (params (Rotation :type Float%20%28single-precision%29))
  (return (select (> Rotation 0.0) (Math|Float|MapRangeClamped Rotation 0.0 1.8e+02 0.0 -0.5) (Math|Float|MapRangeClamped Rotation 0.0 -1.8e+02 0.0 0.5))))

(fn UpdateDistancedScope
  (bind _distancedscopesettings (Variables|ScopeSettings|GetDistancedScopeSettings))
  (bind _distancedscopesettings_2 (Variables|ScopeSettings|GetDistancedScopeSettings))
  (bind _distancedscopesettings_3 (Variables|ScopeSettings|GetDistancedScopeSettings))
  (bind _sightsettings (Utilities|Struct|BreakStruct_DistancedScopeMaster _distancedscopesettings_2))
  (bind _rendertargetsettings (Utilities|Struct|BreakStruct_DistancedScopeMaster _distancedscopesettings))
  (bind _scopeinnersettings (Utilities|Struct|BreakStruct_DistancedScopeMaster _distancedscopesettings_3))
  (bind (_x _y) (Math|Vector2D|BreakVector2D (.rendertargetposition _rendertargetsettings)))
  (bind (_x_2 _y_2) (Math|Vector2D|BreakVector2D (.windowposition _scopeinnersettings)))
  (bind (_x_3 _y_3) (Math|Vector2D|BreakVector2D (.positionoffset _sightsettings)))
  ;[0 0 0 1 16] Create Mesh And Dynamic Material
  (CallFunction|CreateScopeMesh)
  (CallFunction|CreateDynamicMaterial)
  ;[0 0 0 1 16] Create Scene Capture Component
  (Utilities|IsValid (Variables|Default|GetScopeRenderTarget)
    (:Is%20Valid
      _)
    (:Is%20Not%20Valid
      (bind _returnvalue (AddComponent|AddSceneCaptureComponent2D false))
      (Variables|Default|SetScopeRenderTarget _returnvalue)))
  (Transformation|AttachComponentToComponent (Variables|Default|GetScopeRenderTarget) (Variables|Default|GetScopeMeshComponent) "RenderTarget" "SnapToTarget" "KeepWorld" "KeepRelative" true)
  ;[0 0 0 1 16] Update Default FOV
  (Variables|/Script/Engine.SceneCaptureComponent2D|SetFOVAngle (Variables|Default|GetScopeRenderTarget) (Utilities|Struct|BreakStruct_DFOVSettings (.FieldOfViewSettings (Utilities|Struct|BreakStruct_DistancedScopeMaster (Variables|ScopeSettings|GetDistancedScopeSettings)))))
  ;[0 0 0 1 16] Update Render Target Settings
  (Rendering|Material|SetVectorParameterValue (Variables|DynamicMaterials|GetScopeDynamicMaterial) "Glass Color" (.glasscolor _rendertargetsettings) :!class /Script/Engine.MaterialInstanceDynamic)
  (Rendering|Material|SetScalarParameterValue (Variables|DynamicMaterials|GetScopeDynamicMaterial) "Render Target Position X" _x :!class /Script/Engine.MaterialInstanceDynamic)
  (Rendering|Material|SetScalarParameterValue (Variables|DynamicMaterials|GetScopeDynamicMaterial) "Render Target Position Y" _y :!class /Script/Engine.MaterialInstanceDynamic)
  (Rendering|Material|SetScalarParameterValue (Variables|DynamicMaterials|GetScopeDynamicMaterial) "Target Scale" (.rendertargetscale _rendertargetsettings) :!class /Script/Engine.MaterialInstanceDynamic)
  (Rendering|Material|SetScalarParameterValue (Variables|DynamicMaterials|GetScopeDynamicMaterial) "Render Target Rotation" (Demo|SelectRotation (.rendertargetrotation _rendertargetsettings)) :!class /Script/Engine.MaterialInstanceDynamic)
  (Rendering|Material|SetTextureParameterValue (Variables|DynamicMaterials|GetScopeDynamicMaterial) "Render Texture" (.rendertargettexture _rendertargetsettings))
  ;[0 0 0 1 16] Update Scope Inner Settings
  (Rendering|Material|SetScalarParameterValue (Variables|DynamicMaterials|GetScopeDynamicMaterial) "Bump Strength" (.bumpstrength _scopeinnersettings) :!class /Script/Engine.MaterialInstanceDynamic)
  (Rendering|Material|SetScalarParameterValue (Variables|DynamicMaterials|GetScopeDynamicMaterial) "Density" (.density _scopeinnersettings) :!class /Script/Engine.MaterialInstanceDynamic)
  (Rendering|Material|SetScalarParameterValue (Variables|DynamicMaterials|GetScopeDynamicMaterial) "Window Radius" (.radius _scopeinnersettings) :!class /Script/Engine.MaterialInstanceDynamic)
  (Rendering|Material|SetScalarParameterValue (Variables|DynamicMaterials|GetScopeDynamicMaterial) "Distance To Fade" (.distancetofade _scopeinnersettings) :!class /Script/Engine.MaterialInstanceDynamic)
  (Rendering|Material|SetScalarParameterValue (Variables|DynamicMaterials|GetScopeDynamicMaterial) "Fade Position X" _x_2 :!class /Script/Engine.MaterialInstanceDynamic)
  (Rendering|Material|SetScalarParameterValue (Variables|DynamicMaterials|GetScopeDynamicMaterial) "Fade Position Y" _y_2 :!class /Script/Engine.MaterialInstanceDynamic)
  (Rendering|Material|SetVectorParameterValue (Variables|DynamicMaterials|GetScopeDynamicMaterial) "Scope Fade Color" (.fadecolor _scopeinnersettings) :!class /Script/Engine.MaterialInstanceDynamic)
  ;[0 0 0 1 16] Update Sight Texture
  (Rendering|Material|SetScalarParameterValue (Variables|DynamicMaterials|GetScopeDynamicMaterial) "Sight Bump Offset" (.bumpstrength _sightsettings) :!class /Script/Engine.MaterialInstanceDynamic)
  (Rendering|Material|SetScalarParameterValue (Variables|DynamicMaterials|GetScopeDynamicMaterial) "Emissive Power" (.emissivepower _sightsettings) :!class /Script/Engine.MaterialInstanceDynamic)
  (Rendering|Material|SetScalarParameterValue (Variables|DynamicMaterials|GetScopeDynamicMaterial) "Sight Texture Rotation" (Demo|SelectRotation (.rotation _sightsettings)) :!class /Script/Engine.MaterialInstanceDynamic)
  (Rendering|Material|SetScalarParameterValue (Variables|DynamicMaterials|GetScopeDynamicMaterial) "Sight Texture Scale" (.scale _sightsettings) :!class /Script/Engine.MaterialInstanceDynamic)
  (Rendering|Material|SetVectorParameterValue (Variables|DynamicMaterials|GetScopeDynamicMaterial) "Sight Red Color" (.redcolor _sightsettings) :!class /Script/Engine.MaterialInstanceDynamic)
  (Rendering|Material|SetVectorParameterValue (Variables|DynamicMaterials|GetScopeDynamicMaterial) "Sight Green Color" (.greencolor _sightsettings) :!class /Script/Engine.MaterialInstanceDynamic)
  (Rendering|Material|SetVectorParameterValue (Variables|DynamicMaterials|GetScopeDynamicMaterial) "Sight Blue Color" (.bluecolor _sightsettings) :!class /Script/Engine.MaterialInstanceDynamic)
  (Rendering|Material|SetScalarParameterValue (Variables|DynamicMaterials|GetScopeDynamicMaterial) "Sight Position X" _x_3 :!class /Script/Engine.MaterialInstanceDynamic)
  (Rendering|Material|SetScalarParameterValue (Variables|DynamicMaterials|GetScopeDynamicMaterial) "Sight Position Y" _y_3 :!class /Script/Engine.MaterialInstanceDynamic)
  (Rendering|Material|SetTextureParameterValue (Variables|DynamicMaterials|GetScopeDynamicMaterial) "Sight Texture" (.sighttexture _sightsettings)))

(fn CreateDynamicMaterial
  (bind _returnvalue (Rendering|Material|CreateDynamicMaterialInstance (Variables|Default|GetScopeMeshComponent) 1 (Utilities|Select :Index (Variables|ScopeSettings|GetScopeType) :NewEnumerator0 0 :NewEnumerator1 "/Game/PlayerLogic/Blueprint/Weapon/RealisticSights/Materials/Master/M_TransparentScopeMaster.M_TransparentScopeMaster" :NewEnumerator2 "/Game/PlayerLogic/Blueprint/Weapon/RealisticSights/Materials/Master/M_DistancedScopeMaster.M_DistancedScopeMaster") "None" :!class /Script/Engine.PrimitiveComponent))
  (Variables|DynamicMaterials|SetScopeDynamicMaterial _returnvalue)
  (return))

(fn CreateScopeMesh
  (Utilities|IsValid (Variables|Default|GetScopeMeshComponent)
    (:Is%20Valid
      _)
    (:Is%20Not%20Valid
      (bind _returnvalue (AddComponent|AddStaticMeshComponent false))
      (Variables|Default|SetScopeMeshComponent _returnvalue)))
  (Components|StaticMesh|SetStaticMesh (Variables|Default|GetScopeMeshComponent) (Utilities|Select :Index (Variables|ScopeSettings|GetScopeType) :NewEnumerator0 0 :NewEnumerator1 (Utilities|Struct|BreakStruct_MasterTransparentScope (Variables|ScopeSettings|GetTransparentScopeSettings)) :NewEnumerator2 (Utilities|Struct|BreakStruct_DistancedScopeMaster (Variables|ScopeSettings|GetDistancedScopeSettings)))))