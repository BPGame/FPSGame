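; Player camera manager that drives the first-person view and aim-down-sights transition for BP_Player.
; BlueprintUpdateCamera uses control rotation and, by ADSValue, narrows FOV and blends location from FPSCamera toward the active weapon's sight socket, adjusted along the socket's forward axis.
; Each tick interpolates a sway offset from clamped turn and look input, with tighter limits in ADS, which is rotated into view space and added to camera location.
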(event Custom|CE_WeaponSway
  (Utilities|IsValid (Variables|Default|GetAs%20BP%20Player)
    (:Is%20Valid
      (Variables|Default|SetSwayOffset (Math|Interpolation|VInterpTo (Variables|Default|GetSwayOffset) "0, 0, 0" (Utilities|Time|GetWorldDeltaSeconds) 8.0))
      (Variables|Default|SetSwayOffset (Math|Interpolation|VInterpTo (Variables|Default|GetSwayOffset) (select (Variables|/Game/PlayerLogic/Blueprint/BP_Player.BP_Player_C|GetADSEnabled (Variables|Default|GetAs%20BP%20Player)) (Utilities|SwayAds) (Utilities|SwayIndle)) (Utilities|Time|GetWorldDeltaSeconds) 5.0)))))

(event EventTick
  (params (DeltaSeconds :type Float%20%28single-precision%29))
  (CallFunction|CEWeaponSway))

(fn ConstructionScript)

(fn BlueprintUpdateCamera
  (params (CameraTarget :type Actor%20Object%20Reference))
  (bind _asbp_player (Utilities|Casting|CastToBP_Player CameraTarget))
  (bind _output_get (Variables|Default|SetAs%20BP%20Player _asbp_player))
  (Utilities|IsValid _output_get
    (:Is%20Valid
      (Utilities|IsValid (Variables|/Game/PlayerLogic/Blueprint/BP_Player.BP_Player_C|GetActiveWeapon (Variables|Default|GetAs%20BP%20Player))
        (:Is%20Valid
          (Variables|Default|SetFinalCameraRotation (Pawn|GetControlRotation (Variables|Default|GetAs%20BP%20Player) :!class /Script/Engine.Pawn))
          (Variables|Default|SetFinalCameraLocation (+ (Math|Vector|Lerp(Vector) (Transformation|GetWorldLocation (Variables|/Game/PlayerLogic/Blueprint/BP_Player.BP_Player_C|GetFPS_Camera (Variables|Default|GetAs%20BP%20Player))) (- (.Location (Math|Transform|BreakTransform (Transformation|GetSocketTransform (Variables|/Game/PlayerLogic/Blueprint/Weapon/BaseWeapon.BaseWeapon_C|GetWeaponMesh (Variables|/Game/PlayerLogic/Blueprint/BP_Player.BP_Player_C|GetActiveWeapon (Variables|Default|GetAs%20BP%20Player))) (Variables|/Game/PlayerLogic/Blueprint/Weapon/BaseWeapon.BaseWeapon_C|GetSightSocket (Variables|/Game/PlayerLogic/Blueprint/BP_Player.BP_Player_C|GetActiveWeapon (Variables|Default|GetAs%20BP%20Player))) "RTS_World"))) (* (Math|Vector|GetForwardVector (.Rotation (Math|Transform|BreakTransform (Transformation|GetSocketTransform (Variables|/Game/PlayerLogic/Blueprint/Weapon/BaseWeapon.BaseWeapon_C|GetWeaponMesh (Variables|/Game/PlayerLogic/Blueprint/BP_Player.BP_Player_C|GetActiveWeapon (Variables|Default|GetAs%20BP%20Player))) (Variables|/Game/PlayerLogic/Blueprint/Weapon/BaseWeapon.BaseWeapon_C|GetSightSocket (Variables|/Game/PlayerLogic/Blueprint/BP_Player.BP_Player_C|GetActiveWeapon (Variables|Default|GetAs%20BP%20Player))) "RTS_World")))) (* (Math|Vector|DotProduct (Math|Vector|Normalize (- (.Location (Math|Transform|BreakTransform (Transformation|GetSocketTransform (Variables|/Game/PlayerLogic/Blueprint/Weapon/BaseWeapon.BaseWeapon_C|GetWeaponMesh (Variables|/Game/PlayerLogic/Blueprint/BP_Player.BP_Player_C|GetActiveWeapon (Variables|Default|GetAs%20BP%20Player))) (Variables|/Game/PlayerLogic/Blueprint/Weapon/BaseWeapon.BaseWeapon_C|GetSightSocket (Variables|/Game/PlayerLogic/Blueprint/BP_Player.BP_Player_C|GetActiveWeapon (Variables|Default|GetAs%20BP%20Player))) "RTS_World"))) (Transformation|GetWorldLocation (Variables|/Game/PlayerLogic/Blueprint/BP_Player.BP_Player_C|GetFPS_Camera (Variables|Default|GetAs%20BP%20Player)))) 0.0) (Math|Vector|GetForwardVector (.Rotation (Math|Transform|BreakTransform (Transformation|GetSocketTransform (Variables|/Game/PlayerLogic/Blueprint/Weapon/BaseWeapon.BaseWeapon_C|GetWeaponMesh (Variables|/Game/PlayerLogic/Blueprint/BP_Player.BP_Player_C|GetActiveWeapon (Variables|Default|GetAs%20BP%20Player))) (Variables|/Game/PlayerLogic/Blueprint/Weapon/BaseWeapon.BaseWeapon_C|GetSightSocket (Variables|/Game/PlayerLogic/Blueprint/BP_Player.BP_Player_C|GetActiveWeapon (Variables|Default|GetAs%20BP%20Player))) "RTS_World"))))) (/ (Math|Vector|VectorLength (- (.Location (Math|Transform|BreakTransform (Transformation|GetSocketTransform (Variables|/Game/PlayerLogic/Blueprint/Weapon/BaseWeapon.BaseWeapon_C|GetWeaponMesh (Variables|/Game/PlayerLogic/Blueprint/BP_Player.BP_Player_C|GetActiveWeapon (Variables|Default|GetAs%20BP%20Player))) (Variables|/Game/PlayerLogic/Blueprint/Weapon/BaseWeapon.BaseWeapon_C|GetSightSocket (Variables|/Game/PlayerLogic/Blueprint/BP_Player.BP_Player_C|GetActiveWeapon (Variables|Default|GetAs%20BP%20Player))) "RTS_World"))) (Transformation|GetWorldLocation (Variables|/Game/PlayerLogic/Blueprint/BP_Player.BP_Player_C|GetFPS_Camera (Variables|Default|GetAs%20BP%20Player))))) 2.5e+02)))) (Variables|/Game/PlayerLogic/Blueprint/BP_Player.BP_Player_C|GetADSValue (Variables|Default|GetAs%20BP%20Player))) (Math|Vector|RotateVector (Variables|Default|GetSwayOffset) (Variables|Default|GetFinalCameraRotation))))
          (return (Variables|Default|GetFinalCameraLocation) (Variables|Default|GetFinalCameraRotation) (Math|Float|Lerp 9e+01 6e+01 (Variables|/Game/PlayerLogic/Blueprint/BP_Player.BP_Player_C|GetADSValue (Variables|Default|GetAs%20BP%20Player))) true))))))